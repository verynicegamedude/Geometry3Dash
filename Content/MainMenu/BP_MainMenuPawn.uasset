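; Main menu pawn that shows a one-time splash screen and then opens the main menu on BeginPlay.
; The BP_MainGM game instance holds the Zastavaka flag, so the splash shows for a few seconds only until that flag is set.
; A parallel Sequence branch waits out the same delay, then adds the menu widget with UI-only input and a visible cursor.
; It also clears the game instance's MainHUD and FPS flags.
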(event `self.ReceiveBeginPlay`
  (bind _returnvalue (`GameplayStatics.GetPlayerController` 0))
  (`|ExecutionSequence`
    (:`then_0`
      (bind _asbp_main_gm (cast `/Game/CubeBP/Blueprints/BP_MainGM` (`GameplayStatics.GetGameInstance`)))
      (if (not (`/Game/CubeBP/Blueprints/BP_MainGM.Zastavaka` _asbp_main_gm))
        (bind _returnvalue_2 (`|CreateWidget` "/Game/UI/UI_Zastavaka.UI_Zastavaka_C"))
        (`UserWidget.AddToViewport` _returnvalue_2 0)
        (`KismetSystemLibrary.Delay` 3.5)
        (`Widget.RemoveFromParent` _returnvalue_2)
        (set `/Game/CubeBP/Blueprints/BP_MainGM.Zastavaka` true _asbp_main_gm)))
    (:`then_1`
      (bind _asbp_main_gm_2 (cast `/Game/CubeBP/Blueprints/BP_MainGM` (`GameplayStatics.GetGameInstance`)))
      (if (not (`/Game/CubeBP/Blueprints/BP_MainGM.Zastavaka` _asbp_main_gm_2))
        (`KismetSystemLibrary.Delay` 3.5))
      (bind _returnvalue_3 (`|CreateWidget` "/Game/MainMenu/UI_MainMenu.UI_MainMenu_C"))
      (`WidgetBlueprintLibrary.SetInputMode_UIOnlyEx` _returnvalue _returnvalue_3)
      (bind _output_get (set `self.Menu_ref` _returnvalue_3))
      (`UserWidget.AddToViewport` _output_get 0)
      (set `PlayerController.bShowMouseCursor` true _returnvalue)
      (set `/Game/CubeBP/Blueprints/BP_MainGM.MainHUD` false _asbp_main_gm_2)
      (set `/Game/CubeBP/Blueprints/BP_MainGM.FPS` false _asbp_main_gm_2))))

(fn `UserConstructionScript`)
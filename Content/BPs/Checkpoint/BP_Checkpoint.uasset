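; BP_Checkpoint is a checkpoint actor that activates when a BP_Cube overlaps its capsule.
; On overlap it plays the HighScore sound and saves the capsule's world location as SpawnTransformLocation on BP_MainGM, which it obtains by casting the Game Instance.
; It then destroys itself and spawns a BP_ChekpointA at that saved location in its place.
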(event `self.Capsule.OnComponentBeginOverlap`
  (params (OverlappedComponent :type "PrimitiveComponent Object Reference") (OtherActor :type "Actor Object Reference") (OtherComp :type "PrimitiveComponent Object Reference") (OtherBodyIndex :type Integer) (bFromSweep :type Boolean) (SweepResult :type "HitResult Structure (by ref)"))
  (cast `/Game/CubeBP/Blueprints/Cube1/BP_Cube` OtherActor)
  (`GameplayStatics.PlaySoundAtLocation` "/Game/Audio/HighScore.HighScore" (`SceneComponent.K2_GetComponentLocation` (`self.Capsule`)) (struct) 1.0 1.0 0.0 null null null)
  (bind _asbp_main_gm (cast `/Game/CubeBP/Blueprints/BP_MainGM` (`GameplayStatics.GetGameInstance`)))
  (bind _output_get (set `/Game/CubeBP/Blueprints/BP_MainGM.Spawn Transform Location` (`SceneComponent.K2_GetComponentLocation` (`self.Capsule`)) _asbp_main_gm))
  (`self.K2_DestroyActor`)
  (`|SpawnActorFromClass` "/Game/Hack_And_Slash_FX/VFX_Niagara/Impacts/BP_ChekpointA.BP_ChekpointA_C" (`KismetMathLibrary.MakeTransform` _output_get) "Undefined" "OverrideRootScale" null null))

(fn `UserConstructionScript`)